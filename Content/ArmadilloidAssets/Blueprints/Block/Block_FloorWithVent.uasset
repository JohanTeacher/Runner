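; Floor block with a vent hazard whose lid and steam effect toggle between on and off states.
; BeginPlay caches the lid's world location, then moves it to the hazard offset without touching steam or collision.
; ActionOn places the lid at the offset, activates Steam and enables lid collision.
; ActionOff returns the lid to its cached position, deactivates Steam and disables collision, with both moves instant and unswept.
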(event `self.ReceiveBeginPlay`
  (bind _ventlid (`self.ventLid`))
  (set `self.startLocation` (`SceneComponent.K2_GetComponentLocation` _ventlid))
  (`SceneComponent.K2_SetWorldLocation` _ventlid (+ (`self.startLocation`) (`self.hazardLocationOffset`)) false false))

(event `self.ReceiveActorBeginOverlap`
  (params (OtherActor :type "Actor Object Reference")))

(event `self.ReceiveTick`
  (params (DeltaSeconds :type "Float (single-precision)")))

(fn `actionOff`
  (`SceneComponent.K2_SetWorldLocation` (`self.ventLid`) (`self.startLocation`) false false)
  (`ActorComponent.Deactivate` (`self.steam`))
  (`PrimitiveComponent.SetCollisionEnabled` (`self.ventLid`) "NoCollision"))

(fn `actionOn`
  (`SceneComponent.K2_SetWorldLocation` (`self.ventLid`) (+ (`self.startLocation`) (`self.hazardLocationOffset`)) false false)
  (`ActorComponent.Activate` (`self.steam`) false)
  (`PrimitiveComponent.SetCollisionEnabled` (`self.ventLid`) "QueryAndPhysics"))

(fn `UserConstructionScript`
  (`parent.UserConstructionScript`))