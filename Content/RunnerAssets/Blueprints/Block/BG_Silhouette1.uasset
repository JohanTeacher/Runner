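; BG_Silhouette1 is a background silhouette actor in the runner game that stays level with the camera vertically.
; Each Tick it copies the Z location of the first player camera manager into its own transform.
; Its X, Y, rotation and scale stay unchanged, and the move is applied without sweep.
; The construction script only calls its parent.
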(event `self.ReceiveBeginPlay`)

(event `self.ReceiveActorBeginOverlap`
  (params (OtherActor :type "Actor Object Reference")))

(event `self.ReceiveTick`
  (params (DeltaSeconds :type "Float (single-precision)"))
  (`self.K2_SetActorTransform` (`KismetMathLibrary.MakeTransform` (`KismetMathLibrary.MakeVector` (.x (.location (`self.GetTransform`))) (.y (.location (`self.GetTransform`))) (.z (.location (`self.GetTransform` (`GameplayStatics.GetPlayerCameraManager` 0))))) (.rotation (`self.GetTransform`)) (.scale (`self.GetTransform`)))))

(fn `UserConstructionScript`
  (`parent.UserConstructionScript`))