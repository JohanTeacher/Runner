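; Treadmill block for a runner game that switches between forward and backward states.
; Tick spins the large gear about its roll axis by RotationSpeed each frame, without delta-time scaling.
; ActionOn and ActionOff set that speed to the forward or backward value and switch the multiplier on the TreadmillSpeedTrigger child actor to match.
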(event `self.ReceiveBeginPlay`)

(event `self.ReceiveActorBeginOverlap`
  (params (OtherActor :type "Actor Object Reference")))

(event `self.ReceiveTick`
  (params (DeltaSeconds :type "Float (single-precision)"))
  (`SceneComponent.K2_AddWorldRotation` (`self.GearLarge`) (`KismetMathLibrary.MakeRotator` (`self.RotationSpeed`)) false false))

(fn `actionOff`
  (set `self.RotationSpeed` (`self.RotationBackward`))
  (bind _astreadmill_speed_trigger (cast `/Game/RunnerAssets/Blueprints/TreadmillSpeedTrigger` (`ChildActorComponent.ChildActor` (`self.TreadmillSpeedTrigger`))))
  (`/Game/RunnerAssets/Blueprints/TreadmillSpeedTrigger.SetMultiplierToBackward` _astreadmill_speed_trigger 0.0))

(fn `actionOn`
  (set `self.RotationSpeed` (`self.RotationForward`))
  (bind _astreadmill_speed_trigger (cast `/Game/RunnerAssets/Blueprints/TreadmillSpeedTrigger` (`ChildActorComponent.ChildActor` (`self.TreadmillSpeedTrigger`))))
  (`/Game/RunnerAssets/Blueprints/TreadmillSpeedTrigger.SetMultiplierToForward` _astreadmill_speed_trigger))

(fn `UserConstructionScript`
  (`parent.UserConstructionScript`))