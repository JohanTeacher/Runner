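; Runner floor block with a steam vent hazard that toggles between an active and an inactive state.
; BeginPlay caches the lid's world location and turns the steam off.
; ActionOn snaps the lid and ValveJumpTrigger to that location plus HazardLocationOffset, starts the steam and enables lid collision.
; ActionOff returns both to the cached location, stops the steam and disables lid collision.
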(event `self.ReceiveBeginPlay`
  (set `self.startLocation` (`SceneComponent.K2_GetComponentLocation` (`self.ventLid`)))
  (`ActorComponent.Deactivate` (`self.steam`)))

(event `self.ReceiveActorBeginOverlap`
  (params (OtherActor :type "Actor Object Reference")))

(event `self.ReceiveTick`
  (params (DeltaSeconds :type "Float (single-precision)")))

(fn `actionOff`
  (bind _startlocation (`self.startLocation`))
  (`SceneComponent.K2_SetWorldLocation` (`self.ventLid`) _startlocation false false)
  (`SceneComponent.K2_SetWorldLocation` (`self.ValveJumpTrigger`) _startlocation false false)
  (`ActorComponent.Deactivate` (`self.steam`))
  (`PrimitiveComponent.SetCollisionEnabled` (`self.ventLid`) "NoCollision"))

(fn `actionOn`
  (bind _returnvalue (+ (`self.startLocation`) (`self.hazardLocationOffset`)))
  (`SceneComponent.K2_SetWorldLocation` (`self.ventLid`) _returnvalue false false)
  (`SceneComponent.K2_SetWorldLocation` (`self.ValveJumpTrigger`) _returnvalue false false)
  (`ActorComponent.Activate` (`self.steam`) false)
  (`PrimitiveComponent.SetCollisionEnabled` (`self.ventLid`) "QueryAndPhysics"))

(fn `UserConstructionScript`
  (`parent.UserConstructionScript`))