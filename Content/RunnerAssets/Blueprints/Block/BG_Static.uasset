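; BG_Static is a runner background actor that stays aligned with the player camera on the world Y and Z axes.
; Each Tick it copies Y and Z from player 0's camera manager, keeping its own X, rotation and scale.
; The move uses no sweep or teleport, and the construction script only calls its parent.
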(event `self.ReceiveBeginPlay`)

(event `self.ReceiveActorBeginOverlap`
  (params (OtherActor :type "Actor Object Reference")))

(event `/Game/RunnerAssets/Blueprints/Block/BG_Silhouette1.ReceiveTick`
  (params (DeltaSeconds :type "Float (single-precision)"))
  (`self.K2_SetActorTransform` (`KismetMathLibrary.MakeTransform` (`KismetMathLibrary.MakeVector` (.x (.location (`self.GetTransform`))) (.y (.location (`self.GetTransform` (`GameplayStatics.GetPlayerCameraManager` 0)))) (.z (.location (`self.GetTransform` (`GameplayStatics.GetPlayerCameraManager` 0))))) (.rotation (`self.GetTransform`)) (.scale (`self.GetTransform`)))))

(fn `UserConstructionScript`
  (`parent.UserConstructionScript`))