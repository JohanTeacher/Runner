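; Kill trigger for the side-scrolling runner that ends the game when it overlaps the SideScrollerCharacter.
; Each tick it follows the player at a Distance offset, holding its height while the player is falling so a drop can reach it.
; On overlap it converts the player's negated Y position to meters, saves that through a GameSaverBP save slot and opens the Death level.
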(event `self.ReceiveBeginPlay`)

(event `self.ReceiveActorBeginOverlap`
  (params (OtherActor :type "Actor Object Reference"))
  (bind _mysaver (`self.mySaver`))
  ;[1 1 1] On Death: Save Meters to File and go to Death Level
  (if (>= (`KismetArrayLibrary.Array_Length` (`self.GetOverlappingActors` "/Game/RunnerAssets/SideScrollerCharacter.SideScrollerCharacter_C")) 1)
    (bind _returnvalue (`GameplayStatics.CreateSaveGameObject` "/Game/RunnerAssets/Blueprints/GameSaverBP.GameSaverBP_C"))
    (bind _asgame_saver_bp (cast `/Game/RunnerAssets/Blueprints/GameSaverBP` _returnvalue))
    (bind _output_get (set `self.mySaver` _asgame_saver_bp))
    (set `/Game/RunnerAssets/Blueprints/GameSaverBP.meters` (/ (* (`KismetMathLibrary.FFloor` (.y (.location (`self.GetTransform` (`GameplayStatics.GetPlayerCharacter` 0))))) -1) 100) _output_get)
    (`GameplayStatics.SaveGameToSlot` _mysaver (`/Game/RunnerAssets/Blueprints/GameSaverBP.SaveSlotName` _mysaver) (`/Game/RunnerAssets/Blueprints/GameSaverBP.userIndex` _mysaver))
    (`GameplayStatics.OpenLevel` "Death")))

(event `/Game/RunnerAssets/Blueprints/Spawners/SpawnBox_Blueprint.ReceiveTick`
  (params (DeltaSeconds :type "Float (single-precision)"))
  (bind _returnvalue (+ (`self.K2_GetActorLocation` (`GameplayStatics.GetPlayerCharacter` 0)) (`self.distance`)))
  ;[1 1 1] Follow player
  (if (`NavMovementComponent.IsFalling` (`Character.CharacterMovement` (`GameplayStatics.GetPlayerCharacter` 0)))
    (`self.K2_SetActorLocation` (`KismetMathLibrary.MakeVector` (.x _returnvalue) (.y _returnvalue) (.z (`self.K2_GetActorLocation`))))
    (else
      (`self.K2_SetActorLocation` _returnvalue))))

(fn `UserConstructionScript`)