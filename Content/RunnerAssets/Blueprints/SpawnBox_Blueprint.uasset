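; Spawn box actor for an endless runner that generates the level ahead of the player from random floor blocks.
; Each tick it moves to the player's location plus a Distance offset and checks whether any Block actor overlaps it.
; If none does, it spawns one of nine block types at the last block's NextPosition, starting from BlockOne on the first spawn.
; Each new block becomes LastBlock, chaining the track piece by piece.
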(event EventBeginPlay)

(event EventActorBeginOverlap
  (params (OtherActor :type Actor%20Object%20Reference)))

(event EventTick
  (params (DeltaSeconds :type Float%20%28single-precision%29))
  (bind _returnvalue (Transformation|GetActorTransform))
  (bind (_location _rotation _scale) (Math|Transform|BreakTransform _returnvalue))
  ;[1 1 1] Follow player
  (Transformation|SetActorTransform (Math|Transform|MakeTransform (+ (.Location (Math|Transform|BreakTransform (Transformation|GetActorTransform (Game|GetPlayerCharacter 0)))) (Variables|Default|Getdistance)) _rotation _scale))
  ;[1 1 1] Spawn blocks
  (if (== (Utilities|Array|Length (Collision|GetOverlappingActors "/Game/RunnerAssets/Blueprints/Block/Block.Block_C" :!class /Script/Engine.Actor)) 0)
    (if (Variables|Default|GetisSpawning)
      (bind _spawnedblock (CallFunction|SpawnRandomizedBlock (Math|Transform|MakeTransform (Transformation|GetWorldLocation (Variables|/Game/RunnerAssets/Blueprints/Block/Block.Block_C|GetnextPosition (Variables|Default|GetlastBlock))))))
      (Variables|Default|SetlastBlock _spawnedblock)
      (else
        (bind _spawnedblock_2 (CallFunction|SpawnRandomizedBlock (Math|Transform|MakeTransform (Transformation|GetWorldLocation (Variables|/Game/RunnerAssets/Blueprints/Block/Block.Block_C|GetnextPosition (Variables|Default|GetBlockOne))))))
        (Variables|Default|SetlastBlock _spawnedblock_2)))
    (Variables|Default|SetisSpawning true)))

(fn ConstructionScript)

(fn SpawnRandomizedBlock
  (params (transform :type Transform))
  (LocalVariables|Settrans transform)
  (switch int (Math|Random|RandomInteger 9)
    (:Default
      (bind _returnvalue (Game|SpawnActorfromClass "/Game/RunnerAssets/Blueprints/Block/Block_FloorLarge.Block_FloorLarge_C" (LocalVariables|Gettrans) "Undefined" 0 0))
      (return _returnvalue))
    (:0
      (bind _returnvalue_2 (Game|SpawnActorfromClass "/Game/RunnerAssets/Blueprints/Block/Block_Basefloor.Block_Basefloor_C" (LocalVariables|Gettrans) "Undefined" 0 0))
      (return _returnvalue_2))
    (:1
      (bind _returnvalue_3 (Game|SpawnActorfromClass "/Game/RunnerAssets/Blueprints/Block/Block_FloorWithVent.Block_FloorWithVent_C" (LocalVariables|Gettrans) "Undefined" 0 0))
      (return _returnvalue_3))
    (:2
      (bind _returnvalue_4 (Game|SpawnActorfromClass "/Game/RunnerAssets/Blueprints/Block/Block_SimpleBox.Block_SimpleBox_C" (LocalVariables|Gettrans) "Undefined" 0 0))
      (return _returnvalue_4))
    (:3
      (bind _returnvalue_5 (Game|SpawnActorfromClass "/Game/RunnerAssets/Blueprints/Block/Block_Basefloor2.Block_Basefloor2_C" (LocalVariables|Gettrans) "Undefined" 0 0))
      (return _returnvalue_5))
    (:4
      (bind _returnvalue_6 (Game|SpawnActorfromClass "/Game/RunnerAssets/Blueprints/Block/Block_Basefloor3.Block_Basefloor3_C" (LocalVariables|Gettrans) "Undefined" 0 0))
      (return _returnvalue_6))
    (:5
      (bind _returnvalue_7 (Game|SpawnActorfromClass "/Game/RunnerAssets/Blueprints/Block/Block_Basefloor4.Block_Basefloor4_C" (LocalVariables|Gettrans) "Undefined" 0 0))
      (return _returnvalue_7))
    (:6
      (bind _returnvalue_8 (Game|SpawnActorfromClass "/Game/RunnerAssets/Blueprints/Block/Block_FloorUp.Block_FloorUp_C" (LocalVariables|Gettrans) "Undefined" 0 0))
      (return _returnvalue_8))
    (:7
      (bind _returnvalue_9 (Game|SpawnActorfromClass "/Game/RunnerAssets/Blueprints/Block/Block_FloorDown.Block_FloorDown_C" (LocalVariables|Gettrans) "Undefined" 0 0))
      (return _returnvalue_9))))