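; Trigger actor in the runner assets that launches the player upward when they overlap it.
; On begin overlap with the player, it calls Jump, plays a loud pipe-hit sound and starts the first Pipe_jump_Blueprint's audio if idle.
; While overlap lasts, Tick moves the player by RaiseCharacterDistance each frame without sweep, so the lift ignores collision and depends on frame rate.
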(event `self.ReceiveBeginPlay`)

(event `self.ReceiveActorBeginOverlap`
  (params (OtherActor :type "Actor Object Reference"))
  (bind _returnvalue (`GameplayStatics.GetPlayerCharacter` 0))
  (if (`self.IsOverlappingActor` _returnvalue)
    (`Character.Jump` _returnvalue)
    (`GameplayStatics.PlaySound2D` "/Game/RunnerAssets/Sound/pipe_hit.pipe_hit" 10.0)
    (bind _outactors (`GameplayStatics.GetAllActorsOfClass` "/Game/RunnerAssets/Blueprints/pipe_jump_Blueprint.pipe_jump_Blueprint_C"))
    (bind _audiocomponent (`AmbientSound.AudioComponent` (`KismetArrayLibrary.Array_Get` _outactors)))
    (if (not (`AudioComponent.IsPlaying` _audiocomponent))
      (`AudioComponent.Play` _audiocomponent 0.0))))

(event `self.ReceiveTick`
  (params (DeltaSeconds :type "Float (single-precision)"))
  (bind _returnvalue (`GameplayStatics.GetPlayerCharacter` 0))
  (if (`self.IsOverlappingActor` (`GameplayStatics.GetPlayerCharacter` 0))
    (`self.K2_SetActorLocation` _returnvalue (+ (`self.K2_GetActorLocation` _returnvalue) (`self.raiseCharacterDistance`)) false false)))

(fn `PlayerIsOverlaping`
  (returns (isOverlaping :type Boolean))
  (return (`self.IsOverlappingActor` (`GameplayStatics.GetPlayerCharacter` 0))))

(fn `UserConstructionScript`)