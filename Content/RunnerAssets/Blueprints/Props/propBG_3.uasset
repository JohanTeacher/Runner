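; Background prop variant for a runner game that spins continuously around its roll axis.
; BeginPlay appends a fixed set of candidate offsets to PossiblePositions, which this graph does not otherwise use.
; Tick adds RotationSpeed to the roll without delta-time scaling and zeroes pitch and yaw, so spin rate depends on frame rate.
; The construction script only calls its parent.
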(event `/Game/RunnerAssets/Blueprints/Props/propBG_1.ReceiveBeginPlay`
  (`KismetArrayLibrary.Array_Append` (`self.possiblePositions`) (`|MakeArray` (0.0 0.0 150.0) (0.0 -150.0 150.0) (0.0 0.0 250.0) (0.0 -250.0 0.0) (0.0 -250.0 600.0) (0.0 -50.0 600.0) (0.0 -350.0 450.0) :!type "Vector Structure")))

(event `self.ReceiveActorBeginOverlap`
  (params (OtherActor :type "Actor Object Reference")))

(event `self.ReceiveTick`
  (params (DeltaSeconds :type "Float (single-precision)"))
  (`self.SetActorRotation` (`KismetMathLibrary.MakeRotator` (+ (.roll (`self.K2_GetActorRotation`)) (`self.rotationSpeed`)))))

(fn `UserConstructionScript`
  (`parent.UserConstructionScript`))