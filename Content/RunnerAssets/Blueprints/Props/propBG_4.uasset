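; Background prop actor for a runner game, a child Blueprint that spins continuously.
; On BeginPlay it appends its own set of offsets to PossiblePositions, which nothing in this graph reads.
; Each Tick it adds RotationSpeed to the actor's roll and zeroes pitch and yaw, so the step depends on frame rate.
; Component-level rotation nodes for PropBG01 are left unconnected, and construction only calls the parent.
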(event `/Game/RunnerAssets/Blueprints/Props/propBG_1.ReceiveBeginPlay`
  (`KismetArrayLibrary.Array_Append` (`self.possiblePositions`) (`|MakeArray` (0.0 0.0 200.0) (0.0 -200.0 200.0) (0.0 0.0 300.0) (0.0 -300.0 0.0) (0.0 -300.0 650.0) (0.0 -100.0 650.0) (0.0 -400.0 500.0) :!type "Vector Structure")))

(event `self.ReceiveActorBeginOverlap`
  (params (OtherActor :type "Actor Object Reference")))

(event `self.ReceiveTick`
  (params (DeltaSeconds :type "Float (single-precision)"))
  (`self.SetActorRotation` (`KismetMathLibrary.MakeRotator` (+ (.roll (`self.K2_GetActorRotation`)) (`self.rotationSpeed`)))))

(fn `UserConstructionScript`
  (`parent.UserConstructionScript`))