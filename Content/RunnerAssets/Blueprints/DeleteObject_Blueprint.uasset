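; An actor for a runner game that trails the player at an offset and destroys whatever it touches.
; Each tick it moves to the first player character's location plus the Distance offset, keeping its own rotation and scale without sweeping.
; Any actor that begins overlapping it is destroyed, with no class or tag filter.
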(event `self.ReceiveBeginPlay`)

(event `self.ReceiveActorBeginOverlap`
  (params (OtherActor :type "Actor Object Reference"))
  (`self.K2_DestroyActor` OtherActor))

(event `/Game/RunnerAssets/Blueprints/SpawnBox_Blueprint.ReceiveTick`
  (params (DeltaSeconds :type "Float (single-precision)"))
  ;[1 1 1] Follow player
  (`self.K2_SetActorTransform` (`KismetMathLibrary.MakeTransform` (+ (.location (`self.GetTransform` (`GameplayStatics.GetPlayerCharacter` 0))) (`self.distance`)) (.rotation (`self.GetTransform`)) (.scale (`self.GetTransform`)))))

(fn `UserConstructionScript`)