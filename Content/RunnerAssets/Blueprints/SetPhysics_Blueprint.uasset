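; Moving destruction actor in a runner that travels alongside the player character and breaks up the level it overlaps.
; On overlap it enables physics on PropBG static meshes, swaps Blocks for spawned Frac_Block actors and destroys PropFG actors.
; Tick matches player velocity and height, switching Y movement to two-thirds of the fastest recorded -Y step when the player stops, sets a record or falls behind it.
; An alternative self-accelerating movement is left unconnected.
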(event `self.ReceiveBeginPlay`)

(event `self.ReceiveActorBeginOverlap`
  (params (OtherActor :type "Actor Object Reference"))
  (bind _overlappingactors (`self.GetOverlappingActors` "/Game/RunnerAssets/Blueprints/Block/Block.Block_C"))
  ;[1 1 1] setphysics and fracturing on colliding objects
  (for _array_element (`self.GetOverlappingActors` "/Game/RunnerAssets/Blueprints/Props/propBG.propBG_C")
    (bind _asprop_bg (cast `/Game/RunnerAssets/Blueprints/Props/propBG` _array_element))
    (for _array_element_2 (`self.K2_GetComponentsByClass` _asprop_bg "/Script/Engine.StaticMeshComponent")
      (`PrimitiveComponent.SetSimulatePhysics` _array_element_2 true)))
  (for _array_element_3 _overlappingactors
    (`|SpawnActorFromClass` "/Game/RunnerAssets/Blueprints/FracturedObjects/Frac_Block.Frac_Block_C" (`KismetMathLibrary.MakeTransform` (`self.K2_GetActorLocation` _array_element_3)) "Undefined" "OverrideRootScale"))
  (`self.K2_DestroyActor` _overlappingactors)
  (`self.K2_DestroyActor` (`self.GetOverlappingActors` "/Game/RunnerAssets/Blueprints/Props/propFG.propFG_C")))

(event `self.ReceiveTick`
  (params (DeltaSeconds :type "Float (single-precision)"))
  (bind _returnvalue (`GameplayStatics.GetPlayerCharacter` 0))
  (bind _returnvalue_2 (`self.GetVelocity` _returnvalue))
  (bind _z (.z (`self.K2_GetActorLocation` _returnvalue)))
  (bind _returnvalue_3 (* _returnvalue_2 (`KismetMathLibrary.Conv_DoubleToVector` DeltaSeconds)))
  (bind _y (.y _returnvalue_3))
  ;[1 1 1] Tick: Movement and acceleration based on character velocity
  (if (or (== _returnvalue_2 (0.0 0.0 0.0)) (<= (.y (`self.K2_GetActorLocation`)) (.y (`self.K2_GetActorLocation` _returnvalue))))
    (`self.K2_SetActorLocation` (`KismetMathLibrary.MakeVector` (.x (+ (`KismetMathLibrary.MakeVector` (.x _returnvalue_3) (/ (`self.fastest`) 1.5) (.z _returnvalue_3)) (.location (`self.GetTransform`)))) (.y (+ (`KismetMathLibrary.MakeVector` (.x _returnvalue_3) (/ (`self.fastest`) 1.5) (.z _returnvalue_3)) (.location (`self.GetTransform`)))) _z) :!label _label)
    (elif (< _y (`self.fastest`))
      (set `self.fastest` _y)
      (goto _label)
      (else
        (`self.K2_SetActorLocation` (`KismetMathLibrary.MakeVector` (.x (+ _returnvalue_3 (.location (`self.GetTransform`)))) (.y (+ _returnvalue_3 (.location (`self.GetTransform`)))) _z))))))

(fn `UserConstructionScript`)