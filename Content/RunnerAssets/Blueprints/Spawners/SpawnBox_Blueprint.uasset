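; Spawner box for an endless runner that follows the player at a fixed offset and builds the level ahead.
; Whenever it overlaps no Block, it chains a random floor block onto the last one's NextPosition, starting from BlockOne.
; Each new block gets randomized walls, stacked windowless walls below and a randomly placed background prop.
; Past a Y threshold, it occasionally spawns a foreground prop at camera depth and height.
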(event EventBeginPlay)

(event EventActorBeginOverlap
  (params (OtherActor :type Actor%20Object%20Reference)))

(event EventTick
  (params (DeltaSeconds :type Float%20%28single-precision%29))
  (bind _returnvalue (Transformation|GetActorTransform))
  (bind _returnvalue_2 (Game|GetPlayerCameraManager 0))
  (bind (_location _rotation _scale) (Math|Transform|BreakTransform _returnvalue))
  (bind _returnvalue_3 (Transformation|GetActorLocation _returnvalue_2))
  (bind (_x _y _z) (Math|Vector|BreakVector _returnvalue_3))
  ;[1 1 1] Follow player
  (Transformation|SetActorTransform (Math|Transform|MakeTransform (+ (.Location (Math|Transform|BreakTransform (Transformation|GetActorTransform (Game|GetPlayerCharacter 0)))) (Variables|Default|Getdistance)) _rotation _scale))
  ;[1 1 1] Spawn blocks
  (if (== (Utilities|Array|Length (Collision|GetOverlappingActors "/Game/RunnerAssets/Blueprints/Block/Block.Block_C" :!class /Script/Engine.Actor)) 0)
    (if (Variables|Default|GetisSpawning)
      (bind _spawnedblock (CallFunction|SpawnRandomizedBlock (Math|Transform|MakeTransform (Transformation|GetWorldLocation (Variables|/Game/RunnerAssets/Blueprints/Block/Block.Block_C|GetnextPosition (Variables|Default|GetlastBlock))))))
      (Variables|Default|SetlastBlock _spawnedblock)
      (else
        (bind _spawnedblock_2 (CallFunction|SpawnRandomizedBlock (Math|Transform|MakeTransform (Transformation|GetWorldLocation (Variables|/Game/RunnerAssets/Blueprints/Block/Block.Block_C|GetnextPosition (Variables|Default|GetBlockOne))))))
        (Variables|Default|SetlastBlock _spawnedblock_2)))
    (Variables|Default|SetisSpawning true)
    ;[1 1 1] Spawn walls with background props
    (bind _spawnedwall (CallFunction|SpawnRandomizedWalls (Math|Transform|MakeTransform (Transformation|GetWorldLocation (Variables|/Game/RunnerAssets/Blueprints/Block/Block.Block_C|GetwallPosition (Variables|Default|GetlastBlock))))))
    (CallFunction|SpawnRandomizedProp (Math|Transform|MakeTransform (Transformation|GetWorldLocation (Variables|/Game/RunnerAssets/Blueprints/Block/Block.Block_C|GetwallPosition (Variables|Default|GetlastBlock)))))
    ;[1 1 1] Spawn Foreground Props
    (CallFunction|SpawnRandomizedFGProp (Math|Transform|MakeTransform (Math|Vector|MakeVector _x (.Y (Math|Vector|BreakVector (.Location (Math|Transform|BreakTransform (Math|Transform|MakeTransform (Transformation|GetWorldLocation (Variables|/Game/RunnerAssets/Blueprints/Block/Block.Block_C|GetwallPosition (Variables|Default|GetlastBlock)))))))) _z)))
    (CallFunction|SpawnRandomizedWalls (Math|Transform|MakeTransform (Transformation|GetWorldLocation (Variables|/Game/RunnerAssets/Blueprints/Wall/Wall.Wall_C|GettopPosition _spawnedwall))))
    (bind _returnvalue_4 (Game|SpawnActorfromClass "/Game/RunnerAssets/Blueprints/Wall/Wall_Windowless.Wall_Windowless_C" (Math|Transform|MakeTransform (Transformation|GetWorldLocation (Variables|/Game/RunnerAssets/Blueprints/Wall/Wall.Wall_C|GetbottomPosition _spawnedwall))) "Undefined" 0 0))
    (Game|SpawnActorfromClass "/Game/RunnerAssets/Blueprints/Wall/Wall_Windowless.Wall_Windowless_C" (Math|Transform|MakeTransform (Transformation|GetWorldLocation (Variables|/Game/RunnerAssets/Blueprints/Wall/Wall.Wall_C|GetbottomPosition _returnvalue_4))) "Undefined" 0 0)))

(fn ConstructionScript)

(fn SpawnRandomizedProp
  (params (transform :type Transform))
  (LocalVariables|Settrans transform)
  (switch int (Math|Random|RandomInteger 7)
    (:0
      (bind _returnvalue (Game|SpawnActorfromClass "/Game/RunnerAssets/Blueprints/Props/propBG_1.propBG_1_C" (LocalVariables|Gettrans) "Undefined" 0 0))
      (LocalVariables|Setprop _returnvalue))
    (:1
      (bind _returnvalue_2 (Game|SpawnActorfromClass "/Game/RunnerAssets/Blueprints/Props/propBG_2.propBG_2_C" (LocalVariables|Gettrans) "Undefined" 0 0))
      (LocalVariables|Setprop _returnvalue_2))
    (:2
      (bind _returnvalue_3 (Game|SpawnActorfromClass "/Game/RunnerAssets/Blueprints/Props/propBG_3.propBG_3_C" (LocalVariables|Gettrans) "Undefined" 0 0))
      (LocalVariables|Setprop _returnvalue_3))
    (:3
      (bind _returnvalue_4 (Game|SpawnActorfromClass "/Game/RunnerAssets/Blueprints/Props/propBG_4.propBG_4_C" (LocalVariables|Gettrans) "Undefined" 0 0))
      (LocalVariables|Setprop _returnvalue_4))
    (:4
      (bind _returnvalue_5 (Game|SpawnActorfromClass "/Game/RunnerAssets/Blueprints/Props/propBG_5.propBG_5_C" (LocalVariables|Gettrans) "Undefined" 0 0))
      (LocalVariables|Setprop _returnvalue_5))
    (:5
      (bind _returnvalue_6 (Game|SpawnActorfromClass "/Game/RunnerAssets/Blueprints/Props/propBG_6.propBG_6_C" (LocalVariables|Gettrans) "Undefined" 0 0))
      (LocalVariables|Setprop _returnvalue_6))
    (:6
      (bind _returnvalue_7 (Game|SpawnActorfromClass "/Game/RunnerAssets/Blueprints/Props/propBG_7.propBG_7_C" (LocalVariables|Gettrans) "Undefined" 0 0))
      (LocalVariables|Setprop _returnvalue_7)))
  (Transformation|SetActorLocation (LocalVariables|Getprop) (+ (.Location (Math|Transform|BreakTransform (LocalVariables|Gettrans))) (Utilities|Array|Get(acopy) (Variables|/Game/RunnerAssets/Blueprints/Props/propBG.propBG_C|GetpossiblePositions (LocalVariables|Getprop)) (Math|Random|RandomInteger (Utilities|Array|Length (Variables|/Game/RunnerAssets/Blueprints/Props/propBG.propBG_C|GetpossiblePositions (LocalVariables|Getprop)))))) false false)
  (return (LocalVariables|Getprop)))

(fn SpawnRandomizedWalls
  (params (transform :type Transform))
  (LocalVariables|Settrans transform)
  (switch int (Math|Random|RandomInteger 3)
    (:Default
      (bind _returnvalue (Game|SpawnActorfromClass "/Game/RunnerAssets/Blueprints/Wall/Wall_BiggestWindow.Wall_BiggestWindow_C" (LocalVariables|Gettrans) "Undefined" 0 0))
      (return _returnvalue))
    (:0
      (bind _returnvalue_2 (Game|SpawnActorfromClass "/Game/RunnerAssets/Blueprints/Wall/Wall_Windowless.Wall_Windowless_C" (LocalVariables|Gettrans) "Undefined" 0 0))
      (return _returnvalue_2))
    (:1
      (bind _returnvalue_3 (Game|SpawnActorfromClass "/Game/RunnerAssets/Blueprints/Wall/Wall_RoundWindow.Wall_RoundWindow_C" (LocalVariables|Gettrans) "Undefined" 0 0))
      (return _returnvalue_3))
    (:2
      (bind _returnvalue_4 (Game|SpawnActorfromClass "/Game/RunnerAssets/Blueprints/Wall/Wall_BiggestWindow.Wall_BiggestWindow_C" (LocalVariables|Gettrans) "Undefined" 0 0))
      (return _returnvalue_4))))

(fn SpawnRandomizedBlock
  (params (transform :type Transform))
  (LocalVariables|Settrans transform)
  (switch int (Math|Random|RandomInteger 8)
    (:Default
      (bind _returnvalue (Game|SpawnActorfromClass "/Game/RunnerAssets/Blueprints/Block/Block_FloorUp.Block_FloorUp_C" (LocalVariables|Gettrans) "Undefined" 0 0))
      (return _returnvalue))
    (:0
      (bind _returnvalue_2 (Game|SpawnActorfromClass "/Game/RunnerAssets/Blueprints/Block/Block_Basefloor.Block_Basefloor_C" (LocalVariables|Gettrans) "Undefined" 0 0))
      (return _returnvalue_2))
    (:1
      (bind _returnvalue_3 (Game|SpawnActorfromClass "/Game/RunnerAssets/Blueprints/Block/Block_FloorWithVent.Block_FloorWithVent_C" (LocalVariables|Gettrans) "Undefined" 0 0))
      (return _returnvalue_3))
    (:2
      (bind _returnvalue_4 (Game|SpawnActorfromClass "/Game/RunnerAssets/Blueprints/Block/Block_FloorWithVent2.Block_FloorWithVent2_C" (LocalVariables|Gettrans) "Undefined" 0 0))
      (return _returnvalue_4))
    (:3
      (bind _returnvalue_5 (Game|SpawnActorfromClass "/Game/RunnerAssets/Blueprints/Block/Block_Basefloor2.Block_Basefloor2_C" (LocalVariables|Gettrans) "Undefined" 0 0))
      (return _returnvalue_5))
    (:4
      (bind _returnvalue_6 (Game|SpawnActorfromClass "/Game/RunnerAssets/Blueprints/Block/Block_Basefloor3.Block_Basefloor3_C" (LocalVariables|Gettrans) "Undefined" 0 0))
      (return _returnvalue_6))
    (:5
      (bind _returnvalue_7 (Game|SpawnActorfromClass "/Game/RunnerAssets/Blueprints/Block/Block_Basefloor4.Block_Basefloor4_C" (LocalVariables|Gettrans) "Undefined" 0 0))
      (return _returnvalue_7))
    (:6
      (bind _returnvalue_8 (Game|SpawnActorfromClass "/Game/RunnerAssets/Blueprints/Block/Block_Basefloor5.Block_Basefloor5_C" (LocalVariables|Gettrans) "Undefined" 0 0))
      (return _returnvalue_8))
    (:7
      (bind _returnvalue_9 (Game|SpawnActorfromClass "/Game/RunnerAssets/Blueprints/Block/Block_FloorDown.Block_FloorDown_C" (LocalVariables|Gettrans) "Undefined" 0 0))
      (return _returnvalue_9))))

(fn SpawnRandomizedFGProp
  (params (transform :type Transform))
  (LocalVariables|Settrans transform)
  (if (< (.Y (Math|Vector|BreakVector (Transformation|GetActorLocation (Game|GetPlayerCharacter 0)))) (LocalVariables|GetstartsToSpawnAfter))
    (switch int (Math|Random|RandomInteger 20)
      (:0
        (bind _returnvalue (Game|SpawnActorfromClass "/Game/RunnerAssets/Blueprints/Props/propFG_1.propFG_1_C" (LocalVariables|Gettrans) "Undefined" 0 0))
        (LocalVariables|Setprop _returnvalue))
      (:1
        (bind _returnvalue_2 (Game|SpawnActorfromClass "/Game/RunnerAssets/Blueprints/Props/propFG_2.propFG_2_C" (LocalVariables|Gettrans) "Undefined" 0 0))
        (LocalVariables|Setprop _returnvalue_2)))
    (Transformation|SetActorLocation (LocalVariables|Getprop) (+ (.Location (Math|Transform|BreakTransform (LocalVariables|Gettrans))) (Variables|/Game/RunnerAssets/Blueprints/Props/propFG.propFG_C|GetdistanceFromCamera (LocalVariables|Getprop))) false false)
    (return (LocalVariables|Getprop))))