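; Background spawner for the runner that keeps extending scrolling BG set 02 ahead of the player.
; Each tick it moves to the player's location plus an offset and, when no BG overlaps it, spawns a piece.
; Pieces chain from the previous one's NextPosition, with the first attached to ObjectOne.
; The spawn function switches between four variants, but its random maximum of 0 always selects the first.
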(event EventBeginPlay
  (Variables|Default|SetstartPosition (Transformation|GetActorLocation)))

(event Collision|EventActorBeginOverlap
  (params (OtherActor :type Actor%20Object%20Reference)))

(event EventTick
  (params (DeltaSeconds :type Float%20%28single-precision%29))
  (bind _returnvalue (Transformation|GetActorTransform))
  (bind (_location _rotation _scale) (Math|Transform|BreakTransform _returnvalue))
  ;[1 1 1] Follow player
  (Transformation|SetActorTransform (Math|Transform|MakeTransform (+ (.Location (Math|Transform|BreakTransform (Transformation|GetActorTransform (Game|GetPlayerCharacter 0)))) (Variables|Default|Getdistance)) _rotation _scale))
  ;[1 1 1] Spawn blocks
  (if (== (Utilities|Array|Length (Collision|GetOverlappingActors "/Game/RunnerAssets/Blueprints/Backgrounds/BG.BG_C" :!class /Script/Engine.Actor)) 0)
    (if (Variables|Default|GetisSpawning)
      (bind _spawnedbg (CallFunction|SpawnRandomizedObject (Math|Transform|MakeTransform (Transformation|GetWorldLocation (Variables|/Game/RunnerAssets/Blueprints/Backgrounds/BG.BG_C|GetnextPosition (Variables|Default|GetlastObject))))))
      (Variables|Default|SetlastObject _spawnedbg)
      (else
        (bind _spawnedbg_2 (CallFunction|SpawnRandomizedObject (Math|Transform|MakeTransform (Transformation|GetWorldLocation (Variables|/Game/RunnerAssets/Blueprints/Backgrounds/BG.BG_C|GetnextPosition (Variables|Default|GetObjectOne))))))
        (Variables|Default|SetlastObject _spawnedbg_2)))
    (Variables|Default|SetisSpawning true)))

(fn ConstructionScript)

(fn SpawnRandomizedObject
  (params (transform :type Transform))
  (LocalVariables|Settrans transform)
  (switch int (Math|Random|RandomInteger 0)
    (:Default
      (bind _returnvalue (Game|SpawnActorfromClass "/Game/RunnerAssets/Blueprints/Backgrounds/BG_Scrolling_02_04.BG_Scrolling_02_04_C" (LocalVariables|Gettrans) "Undefined" 0 0))
      (return _returnvalue))
    (:0
      (bind _returnvalue_2 (Game|SpawnActorfromClass "/Game/RunnerAssets/Blueprints/Backgrounds/BG_Scrolling_02_01.BG_Scrolling_02_01_C" (LocalVariables|Gettrans) "Undefined" 0 0))
      (return _returnvalue_2))
    (:1
      (bind _returnvalue_3 (Game|SpawnActorfromClass "/Game/RunnerAssets/Blueprints/Backgrounds/BG_Scrolling_02_02.BG_Scrolling_02_02_C" (LocalVariables|Gettrans) "Undefined" 0 0))
      (return _returnvalue_3))
    (:2
      (bind _returnvalue_4 (Game|SpawnActorfromClass "/Game/RunnerAssets/Blueprints/Backgrounds/BG_Scrolling_02_03.BG_Scrolling_02_03_C" (LocalVariables|Gettrans) "Undefined" 0 0))
      (return _returnvalue_4))))