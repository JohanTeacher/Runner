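; Wall spawner for a runner game that extends a chain of randomized wall segments as the player moves.
; Each tick it follows the player's Y at an offset, takes Z from the last spawned block and, when overlapping no Wall, attaches one at the previous wall's RightPosition.
; Helper functions, not called in this graph, spawn randomized background props and occasional foreground props, the latter gated by player Y.
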(event EventBeginPlay)

(event Collision|EventActorBeginOverlap
  (params (OtherActor :type Actor%20Object%20Reference)))

(event EventTick
  (params (DeltaSeconds :type Float%20%28single-precision%29))
  ;[1 1 1] Follow player
  (Transformation|SetActorLocation (Math|Vector|MakeVector (.X (Math|Vector|BreakVector (Transformation|GetActorLocation))) (.Y (Math|Vector|BreakVector (+ (.Location (Math|Transform|BreakTransform (Transformation|GetActorTransform (Game|GetPlayerCharacter 0)))) (Variables|Default|Getdistance)))) (.Z (Math|Vector|BreakVector (Transformation|GetWorldLocation (Variables|/Game/RunnerAssets/Blueprints/Block/Block.Block_C|GetnextPosition (Variables|/Game/RunnerAssets/Blueprints/Spawners/SpawnBox_Blueprint.SpawnBox_Blueprint_C|GetlastBlock (Variables|Default|GetSpawnBox_BP))))))) false false)
  ;[1 1 1] Spawn walls
  (if (== (Utilities|Array|Length (Collision|GetOverlappingActors "/Game/RunnerAssets/Blueprints/Wall/Wall.Wall_C" :!class /Script/Engine.Actor)) 0)
    (if (Variables|Default|GetisSpawning)
      (bind _spawnedwall (CallFunction|SpawnRandomizedWalls (Math|Transform|MakeTransform (Transformation|GetWorldLocation (Variables|/Game/RunnerAssets/Blueprints/Wall/Wall.Wall_C|GetrightPosition (Variables|Default|GetlastWall))))))
      (Variables|Default|SetlastWall _spawnedwall)
      (else
        (bind _spawnedwall_2 (CallFunction|SpawnRandomizedWalls (Math|Transform|MakeTransform (Transformation|GetWorldLocation (Variables|/Game/RunnerAssets/Blueprints/Wall/Wall.Wall_C|GetrightPosition (Variables|Default|GetWallOne))))))
        (Variables|Default|SetlastWall _spawnedwall_2)))
    (Variables|Default|SetisSpawning true)))

(fn ConstructionScript)

(fn SpawnRandomizedProp
  (params (transform :type Transform))
  (LocalVariables|Settrans transform)
  (switch int (Math|Random|RandomInteger 7)
    (:0
      (bind _returnvalue (Game|SpawnActorfromClass "/Game/RunnerAssets/Blueprints/Props/propBG_1.propBG_1_C" (LocalVariables|Gettrans) "Undefined" 0 0))
      (LocalVariables|Setprop _returnvalue))
    (:1
      (bind _returnvalue_2 (Game|SpawnActorfromClass "/Game/RunnerAssets/Blueprints/Props/propBG_2.propBG_2_C" (LocalVariables|Gettrans) "Undefined" 0 0))
      (LocalVariables|Setprop _returnvalue_2))
    (:2
      (bind _returnvalue_3 (Game|SpawnActorfromClass "/Game/RunnerAssets/Blueprints/Props/propBG_3.propBG_3_C" (LocalVariables|Gettrans) "Undefined" 0 0))
      (LocalVariables|Setprop _returnvalue_3))
    (:3
      (bind _returnvalue_4 (Game|SpawnActorfromClass "/Game/RunnerAssets/Blueprints/Props/propBG_4.propBG_4_C" (LocalVariables|Gettrans) "Undefined" 0 0))
      (LocalVariables|Setprop _returnvalue_4))
    (:4
      (bind _returnvalue_5 (Game|SpawnActorfromClass "/Game/RunnerAssets/Blueprints/Props/propBG_5.propBG_5_C" (LocalVariables|Gettrans) "Undefined" 0 0))
      (LocalVariables|Setprop _returnvalue_5))
    (:5
      (bind _returnvalue_6 (Game|SpawnActorfromClass "/Game/RunnerAssets/Blueprints/Props/propBG_6.propBG_6_C" (LocalVariables|Gettrans) "Undefined" 0 0))
      (LocalVariables|Setprop _returnvalue_6))
    (:6
      (bind _returnvalue_7 (Game|SpawnActorfromClass "/Game/RunnerAssets/Blueprints/Props/propBG_7.propBG_7_C" (LocalVariables|Gettrans) "Undefined" 0 0))
      (LocalVariables|Setprop _returnvalue_7)))
  (Transformation|SetActorLocation (LocalVariables|Getprop) (+ (.Location (Math|Transform|BreakTransform (LocalVariables|Gettrans))) (Utilities|Array|Get(acopy) (Variables|/Game/RunnerAssets/Blueprints/Props/propBG.propBG_C|GetpossiblePositions (LocalVariables|Getprop)) (Math|Random|RandomInteger (Utilities|Array|Length (Variables|/Game/RunnerAssets/Blueprints/Props/propBG.propBG_C|GetpossiblePositions (LocalVariables|Getprop)))))) false false)
  (return (LocalVariables|Getprop)))

(fn SpawnRandomizedWalls
  (params (transform :type Transform))
  (LocalVariables|Settrans transform)
  (switch int (Math|Random|RandomInteger 3)
    (:Default
      (bind _returnvalue (Game|SpawnActorfromClass "/Game/RunnerAssets/Blueprints/Wall/Wall_BiggestWindow.Wall_BiggestWindow_C" (LocalVariables|Gettrans) "Undefined" 0 0))
      (return _returnvalue))
    (:0
      (bind _returnvalue_2 (Game|SpawnActorfromClass "/Game/RunnerAssets/Blueprints/Wall/Wall_Windowless.Wall_Windowless_C" (LocalVariables|Gettrans) "Undefined" 0 0))
      (return _returnvalue_2))
    (:1
      (bind _returnvalue_3 (Game|SpawnActorfromClass "/Game/RunnerAssets/Blueprints/Wall/Wall_RoundWindow.Wall_RoundWindow_C" (LocalVariables|Gettrans) "Undefined" 0 0))
      (return _returnvalue_3))
    (:2
      (bind _returnvalue_4 (Game|SpawnActorfromClass "/Game/RunnerAssets/Blueprints/Wall/Wall_BiggestWindow.Wall_BiggestWindow_C" (LocalVariables|Gettrans) "Undefined" 0 0))
      (return _returnvalue_4))))

(fn SpawnRandomizedFGProp
  (params (transform :type Transform))
  (LocalVariables|Settrans transform)
  (if (< (.Y (Math|Vector|BreakVector (Transformation|GetActorLocation (Game|GetPlayerCharacter 0)))) (LocalVariables|GetstartsToSpawnAfter))
    (switch int (Math|Random|RandomInteger 20)
      (:0
        (bind _returnvalue (Game|SpawnActorfromClass "/Game/RunnerAssets/Blueprints/Props/propFG_1.propFG_1_C" (LocalVariables|Gettrans) "Undefined" 0 0))
        (LocalVariables|Setprop _returnvalue))
      (:1
        (bind _returnvalue_2 (Game|SpawnActorfromClass "/Game/RunnerAssets/Blueprints/Props/propFG_2.propFG_2_C" (LocalVariables|Gettrans) "Undefined" 0 0))
        (LocalVariables|Setprop _returnvalue_2)))
    (Transformation|SetActorLocation (LocalVariables|Getprop) (+ (.Location (Math|Transform|BreakTransform (LocalVariables|Gettrans))) (Variables|/Game/RunnerAssets/Blueprints/Props/propFG.propFG_C|GetdistanceFromCamera (LocalVariables|Getprop))) false false)
    (return (LocalVariables|Getprop))))